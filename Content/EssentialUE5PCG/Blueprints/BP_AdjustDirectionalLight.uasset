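; Trigger volume actor that dims the level's directional light while the third-person character is inside its box.
; On BeginPlay it finds a DirectionalLight actor and stores its starting intensity.
; Box overlap begin and end events, filtered by a cast to BP_ThirdPersonCharacter, set a low or high hardcoded intensity.
; The stored default intensity is never read, so exiting does not necessarily restore the original brightness.
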(event `self.ReceiveBeginPlay`
  (bind _returnvalue (`GameplayStatics.GetActorOfClass` "/Script/Engine.DirectionalLight"))
  (set `self.DirectionalLight` _returnvalue)
  (set `self.DefaultLightIntensity` (`LightComponentBase.Intensity` (`Light.LightComponent` (`self.DirectionalLight`)))))

(event `self.Box.OnComponentBeginOverlap`
  (params (OverlappedComponent :type "PrimitiveComponent Object Reference") (OtherActor :type "Actor Object Reference") (OtherComp :type "PrimitiveComponent Object Reference") (OtherBodyIndex :type Integer) (bFromSweep :type Boolean) (SweepResult :type "HitResult Structure (by ref)"))
  ; When Third Person Character enters collision box, turn down directional light intensity
  (cast `/Game/ThirdPerson/Blueprints/BP_ThirdPersonCharacter` OtherActor)
  (`LightComponent.SetIntensity` (`Light.LightComponent` (`self.DirectionalLight`)) 0.1))

(event `self.Box.OnComponentEndOverlap`
  (params (OverlappedComponent :type "PrimitiveComponent Object Reference") (OtherActor :type "Actor Object Reference") (OtherComp :type "PrimitiveComponent Object Reference") (OtherBodyIndex :type Integer))
  ; When Third Person Character enters collision box, turn up directional light intensity
  (cast `/Game/ThirdPerson/Blueprints/BP_ThirdPersonCharacter` OtherActor)
  (`LightComponent.SetIntensity` (`Light.LightComponent` (`self.DirectionalLight`)) 8.0))

(fn `UserConstructionScript`)