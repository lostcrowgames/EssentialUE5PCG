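; PCG dynamic mesh processor that displaces a mesh's surface using a texture map, built on Geometry Script.
; ProcessDynamicMesh first subdivides the incoming mesh with PN tessellation to add vertices, then computes tangents.
; It then applies texture displacement, with magnitude, center, UV scale and offset, and image channel exposed as variables alongside the texture and tessellation level.
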(fn ProcessDynamicMesh
  (params (InDynMesh :type Dynamic%20Mesh%20Object%20Reference))
  (bind _returnvalue (Class|GeometryScriptLibraryMeshSubdivideFunctions|ApplyPNTessellation :TargetMesh InDynMesh :TessellationLevel (Variables|Default|GetTessellation%20Level) :Debug 0))
  (bind _returnvalue_2 (Class|GeometryScriptLibraryMeshNormalsFunctions|ComputeTangents :TargetMesh _returnvalue :Debug 0))
  (Class|GeometryScriptLibraryMeshDeformFunctions|ApplyDisplacefromTextureMap :TargetMesh _returnvalue_2 :Texture (Variables|Default|GetTexture) :Options (Utilities|Struct|MakeGeometryScriptDisplaceFromTextureOptions (Variables|Default|GetMagnitude) (Variables|Default|GetUVScale) (Variables|Default|GetUVOffset) (Variables|Default|GetCenter) (Variables|Default|GetImage%20Channel)) :Debug 0)
  (return 0))