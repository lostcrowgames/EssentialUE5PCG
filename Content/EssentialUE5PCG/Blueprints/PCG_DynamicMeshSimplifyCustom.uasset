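; A custom PCG dynamic mesh element that simplifies an incoming dynamic mesh down to a target vertex count.
; Its ProcessDynamicMesh function passes the mesh to Geometry Script's ApplySimplifyToVertexCount.
; Variables on the element supply the vertex count, simplification method, seam handling, vertex position preservation, quadric memory and auto-compaction options.
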(fn ProcessDynamicMesh
  (params (InDynMesh :type Dynamic%20Mesh%20Object%20Reference))
  (GeometryScript|Simplification|ApplySimplifytoVertexCount InDynMesh (Variables|Default|GetVertexCount) (Utilities|Struct|MakeGeometryScriptSimplifyMeshOptions (Variables|Default|GetMethod) (Variables|Default|GetAllow%20Seam%20Collapse) (Variables|Default|GetAllow%20Seam%20Smoothing) (Variables|Default|GetAllow%20Seam%20Splits) (Variables|Default|GetPreserve%20Vertex%20Positions) (Variables|Default|GetRetain%20Quadric%20Memory) (Variables|Default|GetAuto%20Compact)) 0)
  (return 0))