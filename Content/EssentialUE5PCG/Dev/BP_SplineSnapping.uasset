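; BP_SplineSnapping is a construction-time spline tool that drops spline points onto the surface below or above them.
; When SnapSpline is enabled, the construction script runs SnapPoints and resets a Refresh toggle that serves as a re-run button.
; SnapPoints walks points in reverse, tracing vertically on the Visibility channel and moving each to its hit.
; Point zero, processed last, instead shifts the actor's Z to the hit height.
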(fn `SnapPoints`
  (bind _returnvalue (`SplineComponent.GetLocationAtSplinePoint` (`self.Spline`) (`self.SplinePointIndex`) "World"))
  (for _index (range (- (`SplineComponent.GetNumberOfSplinePoints` (`self.Spline`)) 1) 1)
    (set `self.SplinePointIndex` _index)
    (bind (_outhit _returnvalue_2) (`KismetSystemLibrary.LineTraceSingle` :`Start` (+ _returnvalue (0.0 0.0 1000000.0)) :`End` (- _returnvalue (0.0 0.0 2000000.0)) :`TraceChannel` "TraceTypeQuery1" :`DrawDebugType` "ForDuration"))
    (if _returnvalue_2
      (set `self.Location` (`.Location` (`GameplayStatics.BreakHitResult` _outhit)))
      (if (== (`self.SplinePointIndex`) 0)
        (`self.K2_SetActorLocation` (`KismetMathLibrary.MakeVector` (.x (`self.K2_GetActorLocation`)) (.y (`self.K2_GetActorLocation`)) (.z (`self.Location`))) false true)
        (else
          (`SplineComponent.SetLocationAtSplinePoint` (`self.Spline`) (`self.SplinePointIndex`) (`self.Location`) "World" true)))))
  (return))

(fn `UserConstructionScript`
  (set `self.Refresh` false)
  (if (`self.SnapSpline`)
    (`self.SnapPoints`)))