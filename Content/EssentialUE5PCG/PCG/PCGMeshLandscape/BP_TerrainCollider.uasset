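; BP_TerrainCollider builds collision at runtime for actors tagged StaticMeshLandscape01, apparently the PCG mesh landscape.
; Two seconds after BeginPlay, it loops over those actors and copies each InstancedStaticMeshComponent's mesh into one shared ProceduralMesh with collision enabled.
; When the copy yields sections, it sets that component to query-and-physics collision with a block-all profile.
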(event EventBeginPlay
  (Utilities|FlowControl|Delay 2.0)
  (bind _outactors (Actor|GetAllActorswithTag "StaticMeshLandscape01"))
  (for _array_element _outactors
    (Class|KismetProceduralMeshLibrary|CopyProceduralMeshfromStaticMeshComponent (Actor|GetComponentbyClass _array_element "/Script/Engine.InstancedStaticMeshComponent") 0 (Variables|Default|GetProceduralMesh) true)
    (if (> (Class|ProceduralMeshComponent|GetNumSections (Variables|Default|GetProceduralMesh)) 0)
      (Collision|SetCollisionEnabled (Variables|Default|GetProceduralMesh) "QueryAndPhysics")
      (Collision|SetCollisionProfileName (Variables|Default|GetProceduralMesh) "BLockAll" true :!class /Script/Engine.PrimitiveComponent))))

(fn ConstructionScript)