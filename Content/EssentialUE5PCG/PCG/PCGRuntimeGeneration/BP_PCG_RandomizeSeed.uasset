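; Debug Blueprint that re-rolls the seed of a referenced PCG volume at runtime when the 1 key is pressed.
; It picks a random seed up to a variable maximum, writes it to the volume's PCG component and notifies it of the change.
; It then cleans up and regenerates the PCG output, printing a status message for each step.
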(event Input|KeyboardEvents|1
  (params (Key :type Key%20Structure))
  (bind _pcgvolume (Variables|Default|GetPCGVolume))
  (bind _pcgcomponent (Variables|/Script/PCG.PCGVolume|GetPCGComponent _pcgvolume))
  (:Pressed
    (bind _output_get (Variables|Default|SetSeed (Math|Random|RandomIntegerinRange 0 (Variables|Default|GetRandomInt))))
    (Variables|/Script/PCG.PCGComponent|SetSeed _pcgcomponent _output_get)
    (Class|PCGComponent|NotifyPropertiesChangedfromBlueprint _pcgcomponent)
    (Class|PCGComponent|Cleanup _pcgcomponent false)
    (Development|PrintString "Cleaning up PCG...")
    (Class|PCGComponent|NotifyPropertiesChangedfromBlueprint _pcgcomponent)
    (PCG|Generate _pcgcomponent false)
    (Development|PrintString "Generating PCG...")))

(fn ConstructionScript)