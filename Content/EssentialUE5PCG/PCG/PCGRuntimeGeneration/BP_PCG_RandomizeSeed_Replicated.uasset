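; Blueprint actor that randomizes a PCG volume's seed through a replicated variable, so that generation can follow the server's value.
; Pressing 1 with authority rolls ServerRandomSeed between zero and its current value, while clients only print a debug message.
; The seed's OnRep copies it to ClientRandomSeed and calls Client_GeneratePCG, which applies the seed, then cleans up and regenerates the PCG component.
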(event Custom|Client_GeneratePCG
  (bind _pcgvolume (Variables|Default|GetPCGVolume))
  (bind _pcgcomponent (Variables|/Script/PCG.PCGVolume|GetPCGComponent _pcgvolume))
  (Variables|/Script/PCG.PCGComponent|SetSeed (Variables|/Script/PCG.PCGVolume|GetPCGComponent (Variables|Default|GetPCGVolume)) (Variables|Default|GetServerRandomSeed))
  (Class|PCGComponent|NotifyPropertiesChangedfromBlueprint _pcgcomponent)
  (Class|PCGComponent|Cleanup _pcgcomponent false)
  (Development|PrintString "Cleaning up PCG..." true true "(R=0.000000,G=0.660000,B=1.000000,A=1.000000)" 5.0)
  (Class|PCGComponent|NotifyPropertiesChangedfromBlueprint _pcgcomponent)
  (PCG|Generate _pcgcomponent true)
  (Development|PrintString "Generating PCG..." true true "(R=0.000000,G=0.660000,B=1.000000,A=1.000000)" 5.0))

(event EventTick
  (params (DeltaSeconds :type Float%20%28single-precision%29))
  (Utilities|FlowControl|Delay 3.0)
  (Development|PrintString (Utilities|String|ToString(Integer) (Variables|Default|GetClientRandomSeed))))

(event Input|KeyboardEvents|1
  (params (Key :type Key%20Structure))
  (:Pressed
    (Networking|SwitchHasAuthority
      (:Authority
        (Variables|Default|SetServerRandomSeed (Math|Random|RandomIntegerinRange 0 (Variables|Default|GetServerRandomSeed))))
      (:Remote
        (Development|PrintString "No Server Authority (Client)" true true "(R=1.000000,G=0.000000,B=0.008114,A=1.000000)")
        (Development|PrintString (Utilities|String|ToString(Integer) (Variables|Default|GetClientRandomSeed)))))))

(fn ConstructionScript)

(fn OnRepServerRandomSeed
  (Development|PrintString (Utilities|String|Append "Server Random Seed: " (Utilities|String|ToString(Integer) (Variables|Default|GetServerRandomSeed))))
  (bind _output_get (Variables|Default|SetClientRandomSeed (Variables|Default|GetServerRandomSeed)))
  (Development|PrintString (Utilities|String|Append "Client Random Seed: " (Utilities|String|ToString(Integer) _output_get)))
  (CallFunction|ClientGeneratePCG))