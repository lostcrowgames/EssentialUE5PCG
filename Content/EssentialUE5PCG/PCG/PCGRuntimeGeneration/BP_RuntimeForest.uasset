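; BP_RuntimeForest is an actor that gives debug keyboard control over runtime PCG generation, named for a forest.
; Keys 1, 2 and 3 clean up the referenced PCG, randomize its seed and generate it, each printing a message.
; A new seed does not trigger regeneration by itself.
; The printed seed comes from a separate random evaluation, so it can differ from the assigned one.
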(event EventBeginPlay)

(event Collision|EventActorBeginOverlap
  (params (OtherActor :type Actor%20Object%20Reference)))

(event EventTick
  (params (DeltaSeconds :type Float%20%28single-precision%29)))

(event Input|KeyboardEvents|1
  (params (Key :type Key%20Structure :default "None"))
  (:Pressed
    (Development|PrintString "Clean up PCG")
    (bind _pcg (Variables|Default|GetPCG)
      (:then
        (Class|PCGComponent|Cleanup _pcg true))
      (:else))))

(event Input|KeyboardEvents|3
  (params (Key :type Key%20Structure :default "None"))
  (:Pressed
    (Development|PrintString "Generating PCG")
    (bind _pcg (Variables|Default|GetPCG)
      (:then
        (PCG|Generate _pcg true))
      (:else))))

(event Input|KeyboardEvents|2
  (params (Key :type Key%20Structure :default "None"))
  (bind _randomint (Variables|Default|GetRandomInt))
  (bind _returnvalue (Math|Random|RandomIntegerinRange 0 _randomint))
  (:Pressed
    (Development|PrintString "Randomlize PCG Seed")
    (bind _pcg (Variables|Default|GetPCG)
      (:then
        (Variables|/Script/PCG.PCGComponent|SetSeed _pcg _returnvalue)
        (Development|PrintString (Utilities|String|Append "Seed: " (Utilities|String|ToString(Integer) _returnvalue))))
      (:else))))

(fn ConstructionScript)