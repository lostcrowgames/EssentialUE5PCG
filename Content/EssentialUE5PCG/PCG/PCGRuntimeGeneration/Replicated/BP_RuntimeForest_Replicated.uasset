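; Replicated runtime PCG forest actor that keeps procedural generation in step between server and clients through a shared seed.
; On BeginPlay the authority cleans up and randomizes RandomSeed, while clients only print a warning.
; The RandomSeed RepNotify applies the seed to the PCG component and forces generation.
; Debug keys 1 and 2 rerun cleanup or reseeding on the authority, with print strings tracing each step.
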(event Custom|SERVER_PCG_Cleanup
  (Development|PrintString "Clean up PCG")
  (bind _pcg (Variables|Default|GetPCG)
    (:then
      (Class|PCGComponent|Cleanup _pcg true))
    (:else)))

(event Custom|SERVER_PCG_RandomizeSeed
  (Development|PrintString "Randomlize PCG Seed")
  (bind _pcg (Variables|Default|GetPCG)
    (:then
      (Variables|Default|SetRandomSeed (Math|Random|RandomIntegerinRange 0 (Variables|Default|GetRandomInt)))
      (PCG|Generate _pcg false))
    (:else)))

(event Custom|Client_PCG_Generate
  (Development|PrintString "Generating PCG on clients")
  (bind _pcg (Variables|Default|GetPCG)
    (:then
      (Development|PrintString (Utilities|String|Append "Client seed:" (Utilities|String|ToString(Integer) (Variables|Default|GetRandomSeed))))
      (PCG|Generate _pcg true))
    (:else)))

(event EventBeginPlay
  (Networking|SwitchHasAuthority
    (:Authority
      (CallFunction|SERVERPCGCleanup)
      (CallFunction|SERVERPCGRandomizeSeed))
    (:Remote
      (Development|PrintString "Warning: Client has no authority to spawn PCG 
PCG graph should be generating from server."))))

(event Input|KeyboardEvents|1
  (params (Key :type Key%20Structure :default "None"))
  (:Pressed
    (Networking|SwitchHasAuthority
      (:Authority
        (CallFunction|SERVERPCGCleanup)))))

(event Input|KeyboardEvents|2
  (params (Key :type Key%20Structure :default "None"))
  (:Pressed
    (Networking|SwitchHasAuthority
      (:Authority
        (CallFunction|SERVERPCGRandomizeSeed)))))

(fn ConstructionScript)

(fn OnRepRandomSeed
  (bind _randomseed (Variables|Default|GetRandomSeed))
  (Development|PrintString (Utilities|String|Append "Repnotify random seed:" (Utilities|String|ToString(Integer) (Variables|Default|GetRandomSeed))) true true "(R=0.000000,G=1.000000,B=0.195113,A=1.000000)")
  (Development|PrintString (Utilities|String|Append "Generating PCG with seed: " (Utilities|String|ToString(Integer) _randomseed)))
  (bind _pcg (Variables|Default|GetPCG)
    (:then
      (Variables|/Script/PCG.PCGComponent|SetSeed _pcg _randomseed)
      (PCG|Generate _pcg true))
    (:else)))