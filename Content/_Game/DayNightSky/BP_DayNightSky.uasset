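; BP_DayNightSky drives a day/night cycle for sun, moon, height fog and volumetric clouds.
; When enabled, Tick advances a wrapping 24-hour Time that rotates the sun and samples a curve for fog extinction.
; The sun's pitch selects day or night, switching light intensities, fog albedo and cloud tracing distance to hide clouds at night.
; Moon rotation is disabled, and Time's OnRep function is empty.
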(event `self.ReceiveBeginPlay`
  (`ExponentialHeightFogComponent.SetFogDensity` (`ExponentialHeightFog.Component` (`self.ExponentialHeightFog`)) (`self.FogDensity`)))

(event `self.ReceiveTick`
  (params (DeltaSeconds :type "Float (single-precision)"))
  (bind _directionallightsun (`self.DirectionalLightSun`))
  (bind (_returnvalue_roll _returnvalue_pitch) (`KismetMathLibrary.BreakRotator` (`self.K2_GetActorRotation` _directionallightsun)))
  (if (`self.Enabled`)
    (bind _output_get (set `self.Time` (+ (/ DeltaSeconds (`self.TimeScale`)) (`self.Time`))))
    (`KismetSystemLibrary.PrintString` (`KismetStringLibrary.Conv_DoubleToString` _output_get :!enabledstate Disabled) :!enabledstate Disabled)
    ;[1 1 1] If Time is more than 24 (hours) then reset to 0.
    (if (>= _output_get 24.0)
      (set `self.Time` 0.0)
      (else
        ;[1 0.6649 0.2546] Sun Rotation
        ;;[1 1 1] Rotate Directional Light on Y Axis
        (`/Engine/EditorBlueprintResources/StandardMacros.IsValid` _directionallightsun
          (:`Is Valid`
            (`self.K2_SetActorRelativeRotation` _directionallightsun (`KismetMathLibrary.MakeRotator` 0.0 (* (/ (`self.Time`) 24.0) 360.0)) false false)
            (`ExponentialHeightFogComponent.SetVolumetricFogExtinctionScale` (`ExponentialHeightFog.Component` (`self.ExponentialHeightFog`)) (`CurveFloat.GetFloatValue` (`self.CV_FloatDensity`) (`self.Time`)))
            (if (>= _returnvalue_pitch 0.0)
              (`KismetSystemLibrary.PrintString` "Night" :!enabledstate Disabled)
              (`LightComponent.SetIntensity` (`Light.LightComponent` (`self.DirectionalLightSun`)) 0.1)
              (`LightComponent.SetIntensity` (`Light.LightComponent` (`self.DirectionalLightMoon`)) (`self.NightBrightness`))
              (`ExponentialHeightFogComponent.SetVolumetricFogAlbedo` (`ExponentialHeightFog.Component` (`self.ExponentialHeightFog`)) (`self.NightFogColour`))
              ;[1 1 1] Make volumetric clouds disappear at night if thick volumertric fog
              (`VolumetricCloudComponent.SetTracingMaxDistance` (`VolumetricCloud.VolumetricCloudComponent` (`self.VolumetricCloud`)) 0.1)
              (else
                (`KismetSystemLibrary.PrintString` "Day" :!enabledstate Disabled)
                (`LightComponent.SetIntensity` (`Light.LightComponent` (`self.DirectionalLightSun`)) (`self.DayBrightness`))
                (`LightComponent.SetIntensity` (`Light.LightComponent` (`self.DirectionalLightMoon`)) 0.0)
                (`ExponentialHeightFogComponent.SetVolumetricFogAlbedo` (`ExponentialHeightFog.Component` (`self.ExponentialHeightFog`)) (`self.DayFogColour`))
                ;[1 1 1] Make volumetric clouds disappear at night if thick volumertric fog
                (`VolumetricCloudComponent.SetTracingMaxDistance` (`VolumetricCloud.VolumetricCloudComponent` (`self.VolumetricCloud`)) 50.0)))))))))

(fn `OnRep_Time`)

(fn `UserConstructionScript`)